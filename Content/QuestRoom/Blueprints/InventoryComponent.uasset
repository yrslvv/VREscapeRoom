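; Inventory slot collision component that stores a grabbable item released inside it.
; On overlap, it claims one item whose GrabComponent is tagged InventoryPushable, caching its mesh and scale and starting a looping per-frame timer.
; The timer restores scale and default lighting channel while held; on release it disables physics, snaps the item to the slot, including scale, and switches lighting channel.
; End overlap pauses the timer and frees the slot.
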(event `self.ReceiveBeginPlay`
  ;[1 1 1] Binding Events Since The New Class
  (add `self.OnComponentBeginOverlap` (delegate `BeginOverlap`))
  (add `self.OnComponentEndOverlap` (delegate `EndOverlap`)))

(event `EndOverlap` :!signature `self.OnComponentEndOverlap`
  (params (OverlappedComponent :type "PrimitiveComponent Object Reference") (OtherActor :type "Actor Object Reference") (OtherComp :type "PrimitiveComponent Object Reference") (OtherBodyIndex :type Integer))
  (if (== OtherActor (`self.Item`))
    ;[1 1 1] Stopping Timer & Clearing References
    (`KismetSystemLibrary.K2_PauseTimer` null "KeepItemAttached")
    (set `self.Item` null)
    (set `self.ItemMesh` null)))

(event `BeginOverlap` :!signature `self.OnComponentBeginOverlap`
  (params (OverlappedComponent :type "PrimitiveComponent Object Reference") (OtherActor :type "Actor Object Reference") (OtherComp :type "PrimitiveComponent Object Reference") (OtherBodyIndex :type Integer) (bFromSweep :type Boolean) (SweepResult :type "HitResult Structure (by ref)"))
  (bind _returnvalue (`Actor.GetComponentByClass` OtherActor "/Game/VRTemplate/Blueprints/GrabComponent.GrabComponent_C"))
  (bind _returnvalue_2 (`self.GetAttachParent` _returnvalue))
  ;[1 0.9638 0.2314] Validation Of Item
  (`/Engine/EditorBlueprintResources/StandardMacros.IsValid` (`self.Item`)
    (:`Is Not Valid`
      (`/Engine/EditorBlueprintResources/StandardMacros.IsValid` _returnvalue
        (:`Is Valid`
          (if (`self.ComponentHasTag` _returnvalue "InventoryPushable")
            (set `self.ItemGrabComponent` _returnvalue)
            (bind _asstatic_mesh_component (cast `StaticMeshComponent` _returnvalue_2))
            ;[1 0.2708 0.9165] Setting References To Object
            (set `self.ItemScale` (`self.K2_GetComponentScale` _returnvalue_2))
            (set `self.ItemMesh` _asstatic_mesh_component)
            (set `self.Item` (`self.GetOwner` _returnvalue))
            (`KismetSystemLibrary.K2_SetTimerDelegate` (delegate `KeepItemAttached`) (stale `self.ReceiveTick` DeltaSeconds) true)))))))

(event `self.ReceiveTick`
  (params (DeltaSeconds :type "Float (single-precision)")))

(event `KeepItemAttached`
  ;[1 1 1] Attach The Item If Released In The Component & Keep Its Scale If Not
  (if (`/Game/VRTemplate/Blueprints/GrabComponent.bIsHeld` (`self.ItemGrabComponent`))
    ;;[0.04144 1 0.3233] Keeping Its Scale
    (`self.SetWorldScale3D` (`self.ItemMesh`) (`self.ItemScale`))
    (`self.SetLightingChannels` (`self.ItemMesh`) true false false)
    (else
      ;;[1 0 0.04918] Snapping With Changing The Scale To Inventory Component
      (`self.SetSimulatePhysics` (`self.ItemMesh`) false)
      (`Actor.K2_AttachToComponent` (`self.Item`) self "None" "SnapToTarget" "SnapToTarget" "SnapToTarget" true)
      (`self.SetLightingChannels` (`self.ItemMesh`) false true false))))