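; VR desk for the quest room with a drawer the player can slide using a motion controller.
; Grabbing stores the controller and starts a looping timer at frame-delta interval, which dropping pauses.
; Each timer call projects the controller's position onto the segment between the spline's first two points, moving the drawer there with a fixed world-X offset and zeroed world rotation.
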(event `self.ReceiveBeginPlay`)

(event `self.ReceiveTick`
  (params (DeltaSeconds :type "Float (single-precision)")))

(event `self.GrabComponent.OnGrabbed`
  (params (MotionController :type "MotionControllerComponent Object Reference"))
  (set `self.Motion Controller` MotionController)
  (`KismetSystemLibrary.K2_SetTimerDelegate` (delegate `OnDrawerGrabbed`) (stale `self.ReceiveTick` DeltaSeconds) true))

(event `OnDrawerGrabbed`
  (`self.StartChangingPosition` (`self.Drawer`) (`self.Spline`)))

(event `self.GrabComponent.OnDropped`
  (set `self.Motion Controller` null)
  (`KismetSystemLibrary.K2_PauseTimer` null "OnDrawerGrabbed"))

(fn `StartChangingPosition`
  (params (DrawerMesh :type "StaticMeshComponent Object Reference") (Spline :type "SplineComponent Object Reference"))
  (bind (_returnvalue_x _returnvalue_y _returnvalue_z) (`KismetMathLibrary.BreakVector` (`KismetMathLibrary.FindClosestPointOnSegment` (`SceneComponent.K2_GetComponentLocation` (`self.Motion Controller`)) (`SplineComponent.GetLocationAtSplinePoint` Spline 0 "World") (`SplineComponent.GetLocationAtSplinePoint` Spline 1 "World"))))
  (`SceneComponent.K2_SetWorldLocation` DrawerMesh (`KismetMathLibrary.MakeVector` (- _returnvalue_x 20.0) _returnvalue_y _returnvalue_z) false false)
  (`SceneComponent.K2_SetWorldRotation` :`self` DrawerMesh))

(fn `UserConstructionScript`)