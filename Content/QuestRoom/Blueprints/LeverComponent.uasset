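; VR lever component that pitches to follow the grabbing motion controller and fires a one-shot OnTrigger at its limit.
; It binds to the owner's GrabComponent on BeginPlay, printing an error if missing, and runs a looping Rotate timer while held.
; Rotate derives pitch from the controller's position in lever space, clamped between RotationRange and the initial pitch.
; The Saved function holds an alternative symmetric-range version that only prints activation state.
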(event `self.ReceiveBeginPlay`
  (bind _returnvalue (`self.GetOwner`))
  (bind (_relativerotation_roll _relativerotation_pitch) (`KismetMathLibrary.BreakRotator` (`self.RelativeRotation`)))
  (bind _returnvalue_2 (`Actor.GetComponentByClass` _returnvalue "/Game/VRTemplate/Blueprints/GrabComponent.GrabComponent_C"))
  ;[1 0.05208 0.05208] Error Handling (Check If There Is A GrabComponent)
  (`/Engine/EditorBlueprintResources/StandardMacros.IsValid` _returnvalue_2
    (:`Is Valid`
      (set `self.Initial Rotation Y` _relativerotation_pitch)
      (bind _output_get (set `self.LeverGrabComponent` _returnvalue_2))
      (add `/Game/VRTemplate/Blueprints/GrabComponent.OnGrabbed` _output_get (delegate `OnGrab`))
      (add `/Game/VRTemplate/Blueprints/GrabComponent.OnDropped` _output_get (delegate `OnRelease`)))
    (:`Is Not Valid`
      (`KismetSystemLibrary.PrintString` (`KismetStringLibrary.Concat_StrStr` "No Grab Component Detected For " (`KismetSystemLibrary.GetDisplayName` _returnvalue)) true true (struct :`R` 1.0 :`A` 1.0)))))

(event `OnRelease`
  (`KismetSystemLibrary.K2_PauseTimer` null "Rotate")
  (set `self.Motion Controller` null))

(event `OnGrab`
  (params (MotionController :type "MotionControllerComponent Object Reference"))
  (set `self.Motion Controller` MotionController)
  (`KismetSystemLibrary.K2_SetTimerDelegate` (delegate `Rotate`) 0.01 true))

(event `Rotate`
  (bind (_relativerotation_roll _relativerotation_pitch) (`KismetMathLibrary.BreakRotator` (`self.RelativeRotation`)))
  (bind (_returnvalue_location _returnvalue_rotation _returnvalue_scale) (`KismetMathLibrary.BreakTransform` (`self.K2_GetComponentToWorld` self)))
  (bind _returnvalue_location_2 (`KismetMathLibrary.BreakTransform` (`KismetMathLibrary.MakeRelativeTransform` (`self.K2_GetComponentToWorld` (`self.Motion Controller`)) (`KismetMathLibrary.MakeTransform` _returnvalue_location (`KismetMathLibrary.ComposeRotators` _returnvalue_rotation (struct :`Pitch` 90.0)) _returnvalue_scale))))
  (bind (_returnvalue_roll _returnvalue_pitch) (`KismetMathLibrary.BreakRotator` (`KismetMathLibrary.FindLookAtRotation` (`KismetMathLibrary.MakeVector` 0.0) _returnvalue_location_2)))
  (bind _returnvalue (`KismetMathLibrary.FClamp` (+ _relativerotation_pitch _returnvalue_pitch) (`self.RotationRange`) (`self.Initial Rotation Y`)))
  ;[1 1 1] Rotation Logic
  (`self.K2_SetRelativeRotation` (`KismetMathLibrary.MakeRotator` 0.0 _returnvalue))
  (if (`KismetMathLibrary.NearlyEqual_FloatFloat` _returnvalue (`self.RotationRange`) 0.0001)
    (if (not (`self.IsTriggered`))
      (`self.OnTrigger`)
      (set `self.IsTriggered` true))))

(fn `saved`
  (bind _rotationrange (`self.RotationRange`))
  (bind (_returnvalue_location _returnvalue_rotation _returnvalue_scale) (`KismetMathLibrary.BreakTransform` (`self.K2_GetComponentToWorld` self)))
  (bind (_relativerotation_roll _relativerotation_pitch) (`KismetMathLibrary.BreakRotator` (`self.RelativeRotation`)))
  (bind _returnvalue_location_2 (`KismetMathLibrary.BreakTransform` (`KismetMathLibrary.MakeRelativeTransform` (`self.K2_GetComponentToWorld` (`self.Motion Controller`)) (`KismetMathLibrary.MakeTransform` _returnvalue_location (`KismetMathLibrary.ComposeRotators` _returnvalue_rotation (struct :`Roll` -90.0)) _returnvalue_scale))))
  (bind (_returnvalue_roll _returnvalue_pitch) (`KismetMathLibrary.BreakRotator` (`KismetMathLibrary.FindLookAtRotation` (`KismetMathLibrary.MakeVector` 0.0) _returnvalue_location_2)))
  (bind _returnvalue (`KismetMathLibrary.FClamp` (+ _relativerotation_pitch _returnvalue_pitch) (- 0.0 _rotationrange) _rotationrange))
  (`self.K2_SetRelativeRotation` self (`KismetMathLibrary.MakeRotator` 0.0 _returnvalue) false false)
  (if (>= _returnvalue 90.0)
    (`KismetSystemLibrary.PrintString` "Activated")
    (else
      (`KismetSystemLibrary.PrintString` "Deactivated"))))