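; BP_Chest is a VR quest-room chest that starts hidden without collision and toggles both when its referenced button is pressed.
; A BP_Key entering the KeyHole is released from the hand, snapped in and unlocks the chest, then dissolves through a timeline-driven dynamic material and is destroyed.
; Once unlocked, grabbing runs a looping timer that slides the lid along local Y from controller movement, clamped to LidOffset, until dropped.
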(event `self.ReceiveBeginPlay`
  (add `/Game/QuestRoom/Blueprints/BP_Button.OnButtonPressed` (`self.ButtonRef`) (delegate `VisibilityToggle`))
  (set `self.IsOpen?` false)
  (`self.SetActorHiddenInGame` true)
  (`self.SetActorEnableCollision` false))

(event `VisibilityToggle`
  (bind _returnvalue (not (`self.bHidden`)))
  ;[1 1 1] Toggle Visibility Once Light Is Off
  (`self.SetActorHiddenInGame` self _returnvalue)
  (`self.SetActorEnableCollision` self _returnvalue))

(event `self.KeyHole.OnComponentBeginOverlap`
  (params (OverlappedComponent :type "PrimitiveComponent Object Reference") (OtherActor :type "Actor Object Reference") (OtherComp :type "PrimitiveComponent Object Reference") (OtherBodyIndex :type Integer) (bFromSweep :type Boolean) (SweepResult :type "HitResult Structure (by ref)"))
  (bind _keymesh (`/Game/QuestRoom/Blueprints/BP_Key.KeyMesh` (`self.Key`)))
  ;[1 1 1] Checking For The Key In KeyHole
  (bind _asbp_key (cast `/Game/QuestRoom/Blueprints/BP_Key` OtherActor)) ; We can use tags for specific keys, but I have only 1 :)
  (set `self.Key` _asbp_key)
  (bind _grabcomponent (`/Game/QuestRoom/Blueprints/BP_Key.GrabComponent` _asbp_key))
  (set `/Game/VRTemplate/Blueprints/GrabComponent.bSimulateOnDrop` false _grabcomponent)
  (`/Game/VRTemplate/Blueprints/GrabComponent.TryRelease` _grabcomponent)
  (`self.K2_AttachToComponent` _asbp_key (`self.KeyHole`) "None" "SnapToTarget" "SnapToTarget" "KeepWorld" true)
  (set `self.IsOpen?` true)
  (bind _returnvalue (`PrimitiveComponent.CreateDynamicMaterialInstance` _keymesh 0 "/Game/QuestRoom/Materials/MI_Dissolve.MI_Dissolve" "None"))
  (bind _output_get (set `self.DynamicDissolveMat` _returnvalue))
  (`PrimitiveComponent.SetMaterial` _keymesh 0 _output_get)
  (bind (_direction _dissolveamount) (`Timeline|Dissolve`)
    (:`Update`
      (`MaterialInstanceDynamic.SetScalarParameterValue` (`self.DynamicDissolveMat`) "Dissolve" _dissolveamount))
    (:`Finished`
      (`self.K2_DestroyActor` (`self.Key`)))))

(event `self.GrabComponent.OnGrabbed`
  (params (MotionController :type "MotionControllerComponent Object Reference"))
  ;[1 1 1] Setting Initial States And Creating Timer
  (if (`self.IsOpen?`)
    (bind _output_get (set `self.Motion Controller` MotionController))
    ;;[1 0.3104 0.2806] Avoiding Resetting
    (if (== (`self.InitialControllerWorldLoc`) (0.0 0.0 0.0))
      (set `self.InitialControllerWorldLoc` (`SceneComponent.K2_GetComponentLocation` _output_get)))
    ;;[1 0.3104 0.2806] Avoiding Resetting
    (if (== (`self.InitialLidTransform`) (`self.ZeroVector`))
      (set `self.InitialLidTransform` (`SceneComponent.K2_GetComponentToWorld` (`self.Lid`))))
    (`KismetSystemLibrary.K2_SetTimerDelegate` (delegate `MoveLid`) 0.01 true)))

(event `MoveLid`
  (bind _lid (`self.Lid`))
  (bind _initiallidtransform (`self.InitialLidTransform`))
  (bind (_relativelocation_x _relativelocation_y _relativelocation_z) (`KismetMathLibrary.BreakVector` (`SceneComponent.RelativeLocation` _lid)))
  (bind (_returnvalue_x _returnvalue_y) (`KismetMathLibrary.BreakVector` (- (`KismetMathLibrary.InverseTransformLocation` _initiallidtransform (`self.InitialControllerWorldLoc`)) (`KismetMathLibrary.InverseTransformLocation` _initiallidtransform (`SceneComponent.K2_GetComponentLocation` (`self.Motion Controller`))))))
  ;[1 1 1] Lid Move Logic
  (`SceneComponent.K2_SetRelativeLocation` _lid (`KismetMathLibrary.MakeVector` _relativelocation_x (`KismetMathLibrary.FClamp` (* _returnvalue_y -1.0) (* (`self.LidOffset`) -1.0) 0.0) _relativelocation_z) false false))

(event `self.GrabComponent.OnDropped`
  (set `self.Motion Controller` null)
  (`KismetSystemLibrary.K2_PauseTimer` null "MoveLid"))

(fn `UserConstructionScript`)