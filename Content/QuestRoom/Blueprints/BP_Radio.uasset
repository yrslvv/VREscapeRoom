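; VR radio prop with a push button that toggles music, pausing the sound unless the button is green.
; Each tick, a VR pawn overlapping the collision sphere sinks the button toward zero; otherwise it rises to ButtonOffset, which construction also applies to the arrow.
; Bottoming out arms the switch; on the way back up the click plays and, near the bottom, SwitchColor flips material and state, so toggling happens on release.
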(event `self.ReceiveTick`
  (params (DeltaSeconds :type "Float (single-precision)"))
  (bind _buttontop (`self.ButtonTop`))
  (bind _radiosound (`self.RadioSound`))
  (bind _buttontop_2 (`self.ButtonTop`))
  (bind (_relativelocation_x _relativelocation_y _relativelocation_z) (`KismetMathLibrary.BreakVector` (`SceneComponent.RelativeLocation` _buttontop)))
  (bind (_relativelocation_x_2 _relativelocation_y_2 _relativelocation_z_2) (`KismetMathLibrary.BreakVector` (`SceneComponent.RelativeLocation` (`self.ButtonTop`))))
  (bind (_relativelocation_x_3 _relativelocation_y_3 _relativelocation_z_3) (`KismetMathLibrary.BreakVector` (`SceneComponent.RelativeLocation` _buttontop_2)))
  ;[1 1 1] Toggling Music
  (if (`self.IsGreen?`)
    (`AudioComponent.SetPaused` _radiosound false)
    (else
      (`AudioComponent.SetPaused` _radiosound true)))
  (bind _output_get (set `self.CurrentButtonZLocation` _relativelocation_z_2))
  (if (`KismetMathLibrary.NearlyEqual_FloatFloat` _output_get 0.0 0.001)
    (set `self.ReadyToSwitch?` true)
    (else
      ;[1 0.9555 0.1419] Ready To Switch?
      (if (`self.ReadyToSwitch?`)
        ;[1 0 0.04893] Play Sound
        (`GameplayStatics.PlaySound2D` "/Game/QuestRoom/Sounds/Button/onclick.onclick" 1.0 1.0 0.0 null null)
        ;[1 0.9724 0.237] See If Got Back Enough To Change The color
        (if (`KismetMathLibrary.NearlyEqual_FloatFloat` (`self.CurrentButtonZLocation`) 1.0 0.1)
          (`self.SwitchColor`)
          (set `self.ReadyToSwitch?` false)))))
  (if (> (`KismetArrayLibrary.Array_Length` (`PrimitiveComponent.GetOverlappingActors` (`self.SphereCollision`) "/Game/VRTemplate/Blueprints/VRPawn.VRPawn_C")) 0)
    ;[1 1 1] Moving Button
    ;;[0 1 0.04842] Moving Towards
    (`KismetSystemLibrary.MoveComponentTo` _buttontop_2 (`KismetMathLibrary.MakeVector` 0.0 0.0 (`KismetMathLibrary.FClamp` (- _relativelocation_z_3 1.0) 0.0 (`self.ButtonOffset`))) (struct) false false 0.02)
    (else
      ;;[1 0.1946 0.2643] Moving BackWards
      (`KismetSystemLibrary.MoveComponentTo` _buttontop (`KismetMathLibrary.MakeVector` 0.0 0.0 (`KismetMathLibrary.FClamp` (+ _relativelocation_z 1.0) 0.0 (`self.ButtonOffset`))) (struct) false false 0.0001))))

(fn `SwitchColor`
  (if (`self.IsGreen?`)
    (`PrimitiveComponent.SetMaterial` (`self.ButtonTop`) 0 "/Game/VRE/Grippables/Misc/Examples/Button/Button_Mat_Inst.Button_Mat_Inst")
    (set `self.IsGreen?` false)
    (else
      (`PrimitiveComponent.SetMaterial` (`self.ButtonTop`) 0 "/Game/VRE/Grippables/Misc/Examples/Button/M_Button_Green.M_Button_Green")
      (set `self.IsGreen?` true)))
  (return))

(fn `UserConstructionScript`
  (bind _buttonoffset (`self.ButtonOffset`))
  (set `ArrowComponent.ArrowLength` _buttonoffset (`self.Arrow`))
  (`SceneComponent.K2_SetRelativeLocation` (`self.ButtonTop`) (`KismetMathLibrary.MakeVector` 0.0 0.0 _buttonoffset) false false))