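; VR door that stays ungrabbable, with collision off, until IsOpen is set.
; BeginPlay shows the code lock widget on the LockedSide and gives it the password and a door reference.
; Tick restores collision once the door is open.
; Grabbing starts a looping timer that yaws the door from a look-at between motion controller and door, clamped to a half-turn, and dropping requests a timer pause.
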(event `self.ReceiveBeginPlay`
  (bind _codelockwidget1 (`self.CodeLockWidget1`))
  (bind _codelockwidget2 (`self.CodeLockWidget2`))
  (bind _password (`self.Password`))
  ;[1 0 0.08926] Disable Door Collision With Motion Controllers
  (`PrimitiveComponent.SetCollisionEnabled` (`self.Door`) "NoCollision")
  (switch `/Game/QuestRoom/Megascans/3D_Assets/Door/E_LockSide` (`self.LockedSide`)
    (:`NewEnumerator0`
      (`SceneComponent.SetHiddenInGame` _codelockwidget1 false false)
      (bind _aswb_code_lock (cast `/Game/QuestRoom/UI/WB_CodeLock` (`WidgetComponent.GetWidget` _codelockwidget1)))
      (bind _output_get (set `self.CodeLock1` _aswb_code_lock))
      (set `/Game/QuestRoom/UI/WB_CodeLock.CodeDoorRef` self _output_get)
      (set `/Game/QuestRoom/UI/WB_CodeLock.CorrectCode` _password _output_get))
    (:`NewEnumerator1`
      (`SceneComponent.SetHiddenInGame` _codelockwidget2 false false)
      (bind _aswb_code_lock_2 (cast `/Game/QuestRoom/UI/WB_CodeLock` (`WidgetComponent.GetWidget` _codelockwidget2)))
      (bind _output_get_2 (set `self.CodeLock2` _aswb_code_lock_2))
      (set `/Game/QuestRoom/UI/WB_CodeLock.CodeDoorRef` self _output_get_2)
      (set `/Game/QuestRoom/UI/WB_CodeLock.CorrectCode` _password _output_get_2))))

(event `self.ReceiveTick`
  (params (DeltaSeconds :type "Float (single-precision)"))
  (if (`self.IsOpen`)
    ;[0.04791 1 0.1589] Enable Door Collision With Motion Controllers
    (`/Engine/EditorBlueprintResources/StandardMacros.DoOnce` false
      (:`Completed`
        (`PrimitiveComponent.SetCollisionEnabled` (`self.Door`) "QueryAndPhysics")))))

(event `self.DoorGrabComponent.OnGrabbed`
  (params (MotionController :type "MotionControllerComponent Object Reference"))
  ;[1 1 1] Custom Grab Logic
  (set `self.Motion Controller` MotionController)
  (`KismetSystemLibrary.K2_SetTimerDelegate` (delegate `UpdateRotation`) 0.01 true))

(event `UpdateRotation`
  (bind _door (`self.Door`))
  (bind (_returnvalue_roll _returnvalue_pitch _returnvalue_yaw) (`KismetMathLibrary.BreakRotator` (`KismetMathLibrary.FindLookAtRotation` (`SceneComponent.K2_GetComponentLocation` (`self.Motion Controller`)) (`SceneComponent.K2_GetComponentLocation` _door))))
  ;[1 1 1] Updating Door Rotation Relative To Motion Controller Once Grabbed
  (`SceneComponent.K2_SetWorldRotation` _door (`KismetMathLibrary.MakeRotator` 0.0 0.0 (`KismetMathLibrary.ClampAngle` (- _returnvalue_yaw 90.0) -180.0)) false false))

(event `self.DoorGrabComponent.OnDropped`
  ;[1 1 1] Pausing Timer To Avoid Constant Event Tick
  (set `self.Motion Controller` null)
  (`KismetSystemLibrary.K2_PauseTimer` null "UpdateRotation"))

(fn `UserConstructionScript`
  (`SceneComponent.SetHiddenInGame` (`self.CodeLockWidget2`) true false)
  (`SceneComponent.SetHiddenInGame` (`self.CodeLockWidget1`) true false))