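; VR inventory backpack that stays hidden until grabbed by a motion controller through its GrabComponent.
; On grab it stores the controller, reveals the body with shadows, sets itself active and switches collision so only inventory components are interactible.
; On drop it clears the controller and, if a default component is valid, snaps back onto it, hides, deactivates and resets the body's collision object type.
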(event `self.GrabComponent.OnGrabbed`
  (params (MotionController :type "MotionControllerComponent Object Reference"))
  (bind _backpackbody (`self.BackPackBody`))
  (bind _backpackbody_2 (`self.BackPackBody`))
  (set `self.Motion Controller` MotionController)
  (`SceneComponent.SetHiddenInGame` _backpackbody false true)
  (`PrimitiveComponent.SetCastShadow` _backpackbody true)
  ;[1 1 1] Make Inventory Component Interactible Only
  (set `self.IsActivated` true)
  (`PrimitiveComponent.SetCollisionResponseToChannel` _backpackbody_2 "ECC_GameTraceChannel2" "ECR_Ignore")
  (`PrimitiveComponent.SetCollisionObjectType` _backpackbody_2 "ECC_Visibility"))

(event `self.GrabComponent.OnDropped`
  (bind _backpackbody (`self.BackPackBody`))
  (set `self.Motion Controller` null)
  (bind _defaultcomponent (`self.DefaultComponent`)
    (:`then`
      (`self.K2_AttachToComponent` self _defaultcomponent "None" "SnapToTarget" "SnapToTarget" "KeepWorld" true)
      (`SceneComponent.SetHiddenInGame` _backpackbody true true)
      (`PrimitiveComponent.SetCastShadow` _backpackbody false)
      (set `self.IsActivated` false)
      (`PrimitiveComponent.SetCollisionObjectType` (`self.BackPackBody`) "ECC_GameTraceChannel2"))
    (:`else`)))

(fn `UserConstructionScript`
  (`SceneComponent.SetHiddenInGame` (`self.BackPackBody`) true true))