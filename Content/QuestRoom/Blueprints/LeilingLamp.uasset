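; LeilingLamp is a lamp in the QuestRoom that switches its spotlight on and off from a bound button.
; BeginPlay binds the button press event and puts a dynamic material instance on the lamp mesh.
; Each press toggles SpotLight visibility, then plays the TurnOn or TurnOff timeline based on that visibility.
; The timelines drive the material's Intensity parameter to fade the glow, while the spotlight itself switches instantly.
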(event `self.ReceiveBeginPlay`
  (add `/Game/QuestRoom/Blueprints/BP_Button.OnButtonPressed` (`self.Button`) (delegate `CustomEvent`))
  (bind _returnvalue (`KismetMaterialLibrary.CreateDynamicMaterialInstance` "/Game/QuestRoom/Megascans/3D_Assets/LeilingLamp/light.light"))
  (bind _output_get (set `self.LightDynamicMat` _returnvalue))
  (`PrimitiveComponent.SetMaterial` (`self.LeilingLamp`) 2 _output_get))

(event `CustomEvent`
  (bind _spotlight (`self.SpotLight`))
  (bind _lightdynamicmat (`self.LightDynamicMat`))
  (bind _returnvalue (not (`SceneComponent.bVisible` _spotlight)))
  (`SceneComponent.SetVisibility` _spotlight _returnvalue false)
  (if _returnvalue
    ;[1 1 1] Fading Light On/Off
    (bind (_direction _intensity) (`Timeline|TurnOn`)
      (:`Update`
        (`MaterialInstanceDynamic.SetScalarParameterValue` _lightdynamicmat "Intensity" _intensity)))
    (else
      (bind (_direction_2 _intensity_2) (`Timeline|TurnOff`)
        (:`Update`
          (`MaterialInstanceDynamic.SetScalarParameterValue` _lightdynamicmat "Intensity" _intensity_2))))))

(fn `UserConstructionScript`)