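; VR door that unlocks with a BP_Key and swings by following the motion controller that grabs it.
; Door collision starts disabled, and an editable LockedSide picks which keyhole sphere, if any, listens for the key.
; Key overlap enables door collision and snaps the key into the keyhole.
; While grabbed, a looping timer, used instead of Tick, sets clamped yaw toward the controller until release pauses it.
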(event `self.ReceiveBeginPlay`
  ;[1 0 0.08926] Disable Door Collision With Motion Controllers
  (`PrimitiveComponent.SetCollisionEnabled` (`self.Door`) "NoCollision")
  ;[0.9989 1 0] Checking Which KeyHold Is Active For Detecting Key (Instance Editable)
  (switch `/Game/QuestRoom/Megascans/3D_Assets/Door/E_LockSide` (`self.LockedSide`)
    (:`NewEnumerator0`
      (bind _output_get (set `self.ActiveLockedSphereCollision` (`self.Sphere1`)))
      (add `PrimitiveComponent.OnComponentBeginOverlap` _output_get (delegate `BeginOverlapHandling`) :!label _label)
      (add `PrimitiveComponent.OnComponentBeginOverlap` (stale _output_get_2) (delegate `BeginOverlapHandling`)))
    (:`NewEnumerator1`
      (bind _output_get_2 (set `self.ActiveLockedSphereCollision` (`self.Sphere2`)))
      (goto _label))
    (:`NewEnumerator2`
      (set `self.ActiveLockedSphereCollision` null))))

(event `BeginOverlapHandling`
  (params (OverlappedComponent :type "PrimitiveComponent Object Reference") (OtherActor :type "Actor Object Reference") (OtherComp :type "PrimitiveComponent Object Reference") (OtherBodyIndex :type Integer) (bFromSweep :type Boolean) (SweepResult :type "HitResult Structure (by ref)"))
  (bind _doorgrabcomponent (`self.DoorGrabComponent`))
  (bind (_relativelocation_x _relativelocation_y _relativelocation_z) (`KismetMathLibrary.BreakVector` (`SceneComponent.RelativeLocation` (`SceneComponent.GetAttachParent` (`self.ActiveLockedSphereCollision`)))))
  (bind _asbp_key (cast `/Game/QuestRoom/Blueprints/BP_Key` OtherActor))
  ;[1 1 1] Handling Key Collision
  (set `/Game/VRTemplate/Blueprints/GrabComponent.bSimulateOnDrop` false _doorgrabcomponent)
  (`/Game/VRTemplate/Blueprints/GrabComponent.TryRelease` _doorgrabcomponent)
  ;;[0.04791 1 0.1589] Enable Door Collision With Motion Controllers
  (`PrimitiveComponent.SetCollisionEnabled` (`self.Door`) "QueryAndPhysics")
  (bind _output_get (set `self.Key` _asbp_key))
  (`self.K2_AttachToComponent` _output_get (`SceneComponent.GetAttachParent` (`self.ActiveLockedSphereCollision`)) "None" "SnapToTarget" "SnapToTarget" "KeepWorld" true)
  (`SceneComponent.K2_SetRelativeLocation` (`/Game/QuestRoom/Blueprints/BP_Key.KeyMesh` (`self.Key`)) (`KismetMathLibrary.MakeVector` _relativelocation_x _relativelocation_y (- _relativelocation_z 10.0)) false false))

(event `self.DoorGrabComponent.OnGrabbed`
  (params (MotionController :type "MotionControllerComponent Object Reference"))
  ;[1 1 1] Custom Grab Logic
  (set `self.Motion Controller` MotionController)
  (`KismetSystemLibrary.K2_SetTimerDelegate` (delegate `UpdateRotation`) 0.01 true))

(event `UpdateRotation`
  (bind _door (`self.Door`))
  (bind (_returnvalue_roll _returnvalue_pitch _returnvalue_yaw) (`KismetMathLibrary.BreakRotator` (`KismetMathLibrary.FindLookAtRotation` (`SceneComponent.K2_GetComponentLocation` (`self.Motion Controller`)) (`SceneComponent.K2_GetComponentLocation` _door))))
  ;[1 1 1] Updating Door Rotation Relative To Motion Controller Once Grabbed
  (`SceneComponent.K2_SetWorldRotation` _door (`KismetMathLibrary.MakeRotator` 0.0 0.0 (`KismetMathLibrary.ClampAngle` (- _returnvalue_yaw 90.0) -180.0)) false false))

(event `self.DoorGrabComponent.OnDropped`
  ;[1 1 1] Pausing Timer To Avoid Constant Event Tick
  (set `self.Motion Controller` null)
  (`KismetSystemLibrary.K2_PauseTimer` null "UpdateRotation"))

(fn `UserConstructionScript`)