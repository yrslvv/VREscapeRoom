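; BP_CrankWheel is an interactive crank wheel that rotates in response to a motion controller grabbing it.
; Grabbing stores the controller and starts a looping timer that dots the wheel-to-controller direction with the wheel's right vector.
; The scaled, interpolated result drives a local roll each tick.
; Dropping clears the controller and calls a timer pause by function name; the initial rotation is saved but unused.
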(event `self.ReceiveBeginPlay`
  (set `self.InitialWheelRotation` (`SceneComponent.GetSocketRotation` (`self.SM_Interactive_Crank_Wheel`) "None")))

(event `self.GrabComponent.OnGrabbed`
  (params (MotionController :type "MotionControllerComponent Object Reference"))
  ;[1 1 1] Handling Motion Controller Position Relattive To CrankWheel Position
  (set `self.Motion Controller` MotionController)
  (bind _returnvalue (`KismetSystemLibrary.K2_SetTimerDelegate` (delegate `UpdateRotation`) 0.01 true)))

(event `UpdateRotation`
  ;[1 1 1] Handling Motion Controller Position Relattive To CrankWheel Position
  (bind _output_get (set `self.CurrentValue` (`KismetMathLibrary.FInterpTo` (`self.CurrentValue`) (* (`KismetMathLibrary.NormalizeAxis` (`KismetMathLibrary.Dot_VectorVector` (`KismetMathLibrary.Conv_RotatorToVector` (`KismetMathLibrary.FindLookAtRotation` (`SceneComponent.K2_GetComponentLocation` (`self.SM_Interactive_Crank_Wheel`)) (`SceneComponent.K2_GetComponentLocation` (`self.Motion Controller`)))) (`KismetMathLibrary.GetRightVector` (`SceneComponent.K2_GetComponentRotation` (`self.SM_Interactive_Crank_Wheel`))))) 100.0) (`KismetSystemLibrary.K2_GetTimerElapsedTimeHandle` (stale `self.GrabComponent.OnGrabbed` _returnvalue)) 10.0)))
  (`SceneComponent.K2_AddLocalRotation` (`self.SM_Interactive_Crank_Wheel`) (`KismetMathLibrary.MakeRotator` _output_get) false false))

(event `self.GrabComponent.OnDropped`
  ;[1 1 1] Clearing Out The Reference
  (set `self.Motion Controller` null)
  (`KismetSystemLibrary.K2_PauseTimer` null "UpdateRotation"))

(fn `UserConstructionScript`)